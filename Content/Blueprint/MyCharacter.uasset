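; MyCharacter is a selectable character Blueprint with combat stats, turn state and an orbit-and-zoom camera.
; The construction script loads health, attack, heal and shooting distance from a data table row, and selection toggles a decal.
; The mouse wheel steps a clamped zoom level that Tick eases into spring arm length, while right-mouse drag rotates the arm with clamped pitch.
; Turn handling only toggles and prints; movement input is disconnected.
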(event Custom|Turn
  (switch Utilities|FlowControl|Switch|SwitchonTurnEnum (Variables|Default|GetCurrentTurn)
    (:NewEnumerator0
      (Development|PrintString "PlayerTurn"))
    (:NewEnumerator1
      (Development|PrintString "EnemyTurn"))))

(event EventBeginPlay)

(event Collision|EventActorBeginOverlap
  (params (OtherActor :type Actor%20Object%20Reference)))

(event EventTick
  (params (DeltaSeconds :type Float%20%28single-precision%29))
  (bind _springarm (Variables|Default|GetSpringArm))
  ;[1 1 1] Set camera position to zoom
  (Variables|/Script/Engine.SpringArmComponent|SetTargetArmLength _springarm (Math|Interpolation|FInterpTo (Variables|/Script/Engine.SpringArmComponent|GetTargetArmLength _springarm) (+ (Variables|Default|GetinitCameraZoom) (* (* (Variables|Default|GetvalueCameraZoom) (Variables|Default|GetcurrentCameraZoom)) -1.0)) DeltaSeconds 2.0)))

(event EventSelect
  ;[1 1 1] Select
  (Variables|Default|Setselected true)
  (Rendering|SetVisibility (Variables|Default|GetDecalSelection) true false))

(event EventUnSelect
  ;[1 1 1] UnSelect
  (Variables|Default|Setselected false)
  (Rendering|SetVisibility (Variables|Default|GetDecalSelection) false false))

(event Input|AxisEvents|InputAxisLookX
  (params (AxisValue :type Float%20%28single-precision%29))
  ;[1 1 1] Rotation X
  (if (Game|Player|IsInputKeyDown (Game|GetPlayerController 0) "RightMouseButton")
    (bind _asmy_character (Utilities|Casting|CastToMyCharacter (Game|Player|GetPlayerPawn 0)))
    (Transformation|AddWorldRotation (Variables|MyCharacter_C|GetSpringArm _asmy_character) (Math|Rotator|MakeRotator 0.0 0.0 (* AxisValue (Variables|Default|GetvalueCameraRotation))) false false)))

(event Input|AxisEvents|InputAxisLookY
  (params (AxisValue :type Float%20%28single-precision%29))
  ;[1 1 1] Rotation Y
  (if (Game|Player|IsInputKeyDown (Game|GetPlayerController 0) "RightMouseButton")
    (bind _asmy_character (Utilities|Casting|CastToMyCharacter (Game|Player|GetPlayerPawn 0)))
    (Transformation|SetRelativeRotation (Variables|MyCharacter_C|GetSpringArm _asmy_character) (Math|Rotator|MakeRotator (.roll (Variables|/Script/Engine.SceneComponent|GetRelativeRotation (Variables|MyCharacter_C|GetSpringArm _asmy_character))) (Math|Float|Clamp(Float) (+ (.pitch (Variables|/Script/Engine.SceneComponent|GetRelativeRotation (Variables|MyCharacter_C|GetSpringArm _asmy_character))) (* AxisValue (Variables|Default|GetvalueCameraRotation))) -85.0 2.0) (.yaw (Variables|/Script/Engine.SceneComponent|GetRelativeRotation (Variables|MyCharacter_C|GetSpringArm _asmy_character)))) false false)))

(event Input|AxisEvents|InputAxisMoveForward
  (params (AxisValue :type Float%20%28single-precision%29))
  ;[1 1 1] Test Move cam
)

(event Input|AxisEvents|InputAxisMoveRight
  (params (AxisValue :type Float%20%28single-precision%29))
  ;[1 1 1] Test Move cam
)

(event Input|MouseEvents|MouseWheelAxis
  (params (AxisValue :type Float%20%28single-precision%29))
  (bind _maxcamerazoom (Variables|Default|GetmaxCameraZoom))
  (bind _maxcamerazoom_2 (Variables|Default|GetmaxCameraZoom))
  ;[1 1 1] Set value of zoom
  (if (> AxisValue 0.0)
    (bind _result (Math|Integer|IncrementInt (Variables|Default|GetcurrentCameraZoom))
      (:%20%20
        (Variables|Default|SetcurrentCameraZoom (Math|Integer|Clamp(Integer) _result (* _maxcamerazoom_2 -1) _maxcamerazoom_2))))
    (elif (< AxisValue 0.0)
      (bind _result_2 (Math|Integer|DecrementInt (Variables|Default|GetcurrentCameraZoom))
        (:%20%20
          (Variables|Default|SetcurrentCameraZoom (Math|Integer|Clamp(Integer) _result_2 (* _maxcamerazoom -1) _maxcamerazoom)))))))

(fn ConstructionScript
  (bind _data (Variables|Default|GetData))
  (bind (_datatable _rowname) (Utilities|Struct|BreakDataTableRowHandle _data))
  (bind _returnvalue (Utilities|GetDataTableRow _datatable _rowname)
    (:then
      (Variables|Default|SetPV (.hp (Utilities|Struct|BreakS_typePlayer _returnvalue)))
      (Variables|Default|SetAtk (.atk (Utilities|Struct|BreakS_typePlayer _returnvalue)))
      (Variables|Default|SetHeal (.heal (Utilities|Struct|BreakS_typePlayer _returnvalue)))
      (Variables|Default|SetDist_Shoot (.distance_shoot (Utilities|Struct|BreakS_typePlayer _returnvalue))))))

(fn SwitchTurn
  (if (Utilities|Enum|Equal(Enum) (Variables|Default|GetCurrentTurn) "NewEnumerator0")
    (Variables|Default|SetCurrentTurn "NewEnumerator1")
    (else
      (Variables|Default|SetCurrentTurn "NewEnumerator0"))))