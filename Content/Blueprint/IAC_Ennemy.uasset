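; AI controller for enemy characters that prepares their behavior tree and action list.
; InitBehaviorTree runs the tree, seeds the blackboard's ActionPoints from the possessed BP_EnnemyCharacter's maximum, then immediately stops the brain logic, leaving the tree initialized but idle.
; The enemy's Type (DPS, Healer or Tank) selects which action data table becomes its ActionList.
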(event Custom|Init%20BehaviorTree
  (bind _bt (Variables|Default|GetBT))
  ;[1 1 1] Init Behavior Tree and Action in data table
  (AI|RunBehaviorTree _bt)
  (bind _blackboardcomponent (Class|AIController|UseBlackboard (Class|BlackboardAssetProvider|GetBlackboardAsset _bt)))
  (bind _asbp_ennemy_character (Utilities|Casting|CastToBP_EnnemyCharacter (Pawn|GetControlledPawn)))
  (Class|BlackboardComponent|SetValueasInt _blackboardcomponent (Utilities|Name|MakeLiteralName "ActionPoints") (Variables|/Game/Blueprint/BP_EnnemyCharacter.BP_EnnemyCharacter_C|GetMax_ActionPoint _asbp_ennemy_character))
  (AI|Logic|StopLogic (Variables|Default|GetBrainComponent) "Init BT")
  (switch Utilities|FlowControl|Switch|SwitchonE_TypeCharacter (Variables|/Game/Blueprint/BP_EnnemyCharacter.BP_EnnemyCharacter_C|GetType _asbp_ennemy_character)
    (:NewEnumerator0
      (Variables|Default|SetActionList "/Game/Blueprint/Struct/DT_ActionList_DPS.DT_ActionList_DPS"))
    (:NewEnumerator1
      (Variables|Default|SetActionList "/Game/Blueprint/Struct/DT_ActionList_Heal.DT_ActionList_Heal"))
    (:NewEnumerator2
      (Variables|Default|SetActionList "/Game/Blueprint/Struct/DT_ActionList_Tank.DT_ActionList_Tank"))))

(event EventBeginPlay)

(event EventTick
  (params (DeltaSeconds :type Float%20%28single-precision%29)))

(fn ConstructionScript)