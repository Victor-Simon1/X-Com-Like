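; BP_Zone is a clickable map zone, identified by an Id, that serves as a movement target and tracks hero location.
; Clicking its Cube passes the Id to BP_TopDownController2's MovePlayer.
; When a BP_ParentHeros actor begins overlapping the zone, it sets that hero's CurrentZone to the Id, then calls UpdateZone on BP_GameMode.
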(event OnClicked(Cube)
  (params (TouchedComponent :type Primitive%20Component%20Object%20Reference) (ButtonPressed :type Key%20Structure :default "None"))
  ;[1 1 1] When click on zone
  (bind _asbp_top_down_controller_2 (Utilities|Casting|CastToBP_TopDownController2 (Game|GetPlayerController 0)))
  (Default|MovePlayer _asbp_top_down_controller_2 (Variables|Default|Getid)))

(event EventBeginPlay)

(event EventTick
  (params (DeltaSeconds :type Float%20%28single-precision%29)))

(event Collision|EventActorBeginOverlap
  (params (OtherActor :type Actor%20Object%20Reference))
  ;[1 1 1] When heros enter in zone
  (bind _asbp_parent_heros (Utilities|Casting|CastToBP_ParentHeros OtherActor))
  (Variables|/Script/XComLike.XComHerosCharacter|SetcurrentZone _asbp_parent_heros (Variables|Default|Getid))
  (bind _asbp_game_mode (Utilities|Casting|CastToBP_GameMode (Game|GetGameMode)))
  (Default|UpdateZone _asbp_game_mode))

(fn ConstructionScript)