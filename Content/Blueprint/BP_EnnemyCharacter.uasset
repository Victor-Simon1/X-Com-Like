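; Enemy character for a turn-based game, typed as DPS, Healer or Tank and driven by a behavior tree.
; The construction script fills its stats, portrait, type and action points from a data table row.
; On BeginPlay it assigns the behavior tree matching its type to its IAC_Ennemy AI controller and initializes it.
; GiveTurn starts the enemy's turn by restarting that controller's brain logic.
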(event Collision|EventActorBeginOverlap
  (params (OtherActor :type Actor%20Object%20Reference)))

(event EventTick
  (params (DeltaSeconds :type Float%20%28single-precision%29)))

(event EventBeginPlay
  (|CallParentFunction)
  (CallFunction|InitBTinController))

(fn ConstructionScript
  (bind _datatable (Variables|Default|GetdataTable))
  (bind (_datatable_2 _rowname) (Utilities|Struct|BreakDataTableRowHandle _datatable))
  (bind _returnvalue (Utilities|GetDataTableRow _datatable_2 _rowname)
    (:then
      (bind _output_get (Variables|Default|Sethp (.hp (Utilities|Struct|BreakS_typePlayer _returnvalue))))
      (Variables|Default|SethpMax _output_get)
      (Variables|Default|Setatk (.atk (Utilities|Struct|BreakS_typePlayer _returnvalue)))
      (Variables|Default|Setheal (.heal (Utilities|Struct|BreakS_typePlayer _returnvalue)))
      (Variables|Default|SetdistShoot (.distance_shoot (Utilities|Struct|BreakS_typePlayer _returnvalue)))
      (Variables|Default|Setpicture (.picture (Utilities|Struct|BreakS_typePlayer _returnvalue)))
      (Variables|Default|SetType (.type (Utilities|Struct|BreakS_typePlayer _returnvalue)))
      (Variables|Default|SetmaxActionPoint (Math|Conversions|ToInteger(Byte) (.max_point_action (Utilities|Struct|BreakS_typePlayer _returnvalue)))))))

(fn GiveTurn
  (bind _asiac_ennemy (Utilities|Casting|CastToIAC_Ennemy (Pawn|GetController)))
  (Class|BrainComponent|RestartLogic (Variables|/Script/AIModule.AIController|GetBrainComponent _asiac_ennemy)))

(fn InitBTinController
  ;[1 1 1] Put BT in function of the type
  (bind _asiac_ennemy (Utilities|Casting|CastToIAC_Ennemy (Pawn|GetController)))
  (switch Utilities|FlowControl|Switch|SwitchonE_TypeCharacter (Variables|Default|GetType)
    (:NewEnumerator0
      (Variables|/Game/Blueprint/IAC_Ennemy.IAC_Ennemy_C|SetBT _asiac_ennemy "/Game/Blueprint/IA/BehaviorTree/BT_Ennemie_DPS.BT_Ennemie_DPS"))
    (:NewEnumerator1
      (Variables|/Game/Blueprint/IAC_Ennemy.IAC_Ennemy_C|SetBT _asiac_ennemy "/Game/Blueprint/IA/BehaviorTree/BT_Ennemie_Healer.BT_Ennemie_Healer"))
    (:NewEnumerator2
      (Variables|/Game/Blueprint/IAC_Ennemy.IAC_Ennemy_C|SetBT _asiac_ennemy "/Game/Blueprint/IA/BehaviorTree/BT_Ennemie_Tank.BT_Ennemie_Tank")))
  (Default|InitBehaviorTree _asiac_ennemy))