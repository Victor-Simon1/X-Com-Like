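; LogLibrary provides an AddLog function that shows a categorized message in the on-screen log.
; It maps the event type (error, warning or event) to a text prefix and color, then prepends the prefix to the message.
; The result goes to the log box of the first WB_UI widget found by a class search, with a fixed short duration.
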(fn AddLog
  (params (event :type ETypeLog%20Enum :default "tError") (message :type String))
  (switch Utilities|FlowControl|Switch|SwitchonETypeLog event
    (:tError
      (LocalVariables|SetcurrentStr "Error :")
      (LocalVariables|SetcurrentColor ""))
    (:tWarning
      (LocalVariables|SetcurrentStr "Warning : ")
      (LocalVariables|SetcurrentColor ""))
    (:tEvent
      (LocalVariables|SetcurrentStr "Event :")
      (LocalVariables|SetcurrentColor "")))
  (bind _foundwidgets (Widget|GetAllWidgetsOfClass 0 "/Game/Blueprint/Interface/WB_UI.WB_UI_C" false))
  (Default|AddLogMessage (Variables|/Game/Blueprint/Interface/WB_UI.WB_UI_C|GetWB_LogBox (Utilities|Array|Get(acopy) _foundwidgets)) (Utilities|Text|ToText(String) (Utilities|String|Append (Utilities|String|ToString(Text) (LocalVariables|GetcurrentStr)) message)) 1.0 (LocalVariables|GetcurrentColor)))