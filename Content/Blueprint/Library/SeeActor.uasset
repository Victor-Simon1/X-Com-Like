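; SeeActor is a function library of enemy perception and facing helpers.
; SeePlayer tests whether the player lies within a view-cone angle of the enemy's forward vector, without a line trace.
; RotateToActor sets an actor's root rotation toward another through a rotator lerp with no alpha set.
; IsInRange compares 2D distance to a threshold and prints that distance on screen as long-lasting debug text.
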(fn SeePlayer
  (params (Ennemies :type BP%20Ennemy%20Character%20Object%20Reference) (Player :type BP%20Parent%20Heros%20Object%20Reference) (Angle :type Float%20%28double-precision%29))
  (return (< (Class|KismetMathLibrary|DegAcos (Math|Vector|DotProduct (Math|Vector|GetUnitDirection(Vector) (Transformation|GetActorLocation Ennemies) (Transformation|GetActorLocation Player)) (Transformation|GetActorForwardVector Ennemies))) Angle)))

(fn RotatetoActor
  (params (Actor1 :type Actor%20Object%20Reference) (Actor2 :type Actor%20Object%20Reference))
  (Transformation|SetWorldRotation (Variables|/Script/Engine.Actor|GetRootComponent Actor1) (Math|Rotator|Lerp(Rotator) (Math|Rotator|FindLookatRotation (Transformation|GetActorLocation Actor1) (Transformation|GetActorLocation Actor2)) (Transformation|GetWorldRotation (Variables|/Script/Engine.Actor|GetRootComponent Actor1)) 0.0) false false))

(fn IsinRange
  (params (Actor :type Actor%20Object%20Reference) (Actor3 :type Actor%20Object%20Reference) (Distance :type Float%20%28double-precision%29))
  (bind _returnvalue (Transformation|GetActorLocation Actor))
  (bind _returnvalue_2 (Transformation|GetActorLocation Actor3))
  (bind _returnvalue_3 (Math|Vector|Distance2D(Vector) _returnvalue _returnvalue_2))
  (Development|PrintString 0 (Utilities|String|ToString(Float) _returnvalue_3) true true "(R=1.000000,G=0.109378,B=0.000000,A=1.000000)" 2e+03)
  (return (< _returnvalue_3 Distance)))