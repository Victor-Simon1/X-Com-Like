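; AnimLibrary is a function library that plays surface-dependent footstep sounds for the player character.
; FootstepNotify line-traces down from player 0 on the Visibility channel, skipping the supplied actors, and reads the hit's physical surface.
; It plays a grass or concrete cue at the impact with randomized pitch, defaulting to concrete.
; AddIgnoreActors appends every BP_Zone actor to a given array, suitable as the trace's ignore list.
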(fn AddIgnoreActors
  (params (Array :type Array%20of%20BP%20Zone%20Object%20References))
  (bind _outactors (Actor|GetAllActorsOfClass 0 "/Game/Blueprint/Actions/BP_Zone.BP_Zone_C"))
  (for _array_element _outactors
    (Utilities|Array|Add Array _array_element)))

(fn FootstepNotify
  (params (IgnoreActors :type Array%20of%20BP%20Zone%20Object%20References))
  (bind _returnvalue (Game|GetPlayerCharacter 0))
  (bind _returnvalue_2 (Transformation|GetActorLocation _returnvalue))
  (bind (_outhit _returnvalue_3) (Collision|LineTraceByChannel 0 _returnvalue_2 (- _returnvalue_2 "0,0,500.000000") "TraceTypeQuery1" false IgnoreActors "None" true "(R=0.436432,G=0.000000,B=1.000000,A=1.000000)"))
  (if _returnvalue_3
    (switch Utilities|FlowControl|Switch|SwitchonEPhysicalSurface (Collision|GetSurfaceType _outhit)
      (:SurfaceType_Default
        (Audio|PlaySoundatLocation 0 "/Game/LVL/Sound/Step/Concrete/SW_FootStepConcrete_Cue.SW_FootStepConcrete_Cue" (.Location (Collision|BreakHitResult _outhit)) "0, 0, 0" 1.0 (Math|Random|RandomFloatinRange 0.8 1.2) 0.0 0 0 0 0 :!label _label))
      (:SurfaceType1
        (Audio|PlaySoundatLocation 0 "/Game/LVL/Sound/Step/Grass/S_Grass0_Cue.S_Grass0_Cue" (.Location (Collision|BreakHitResult _outhit)) "0, 0, 0" 1.0 (Math|Random|RandomFloatinRange 0.8 1.2) 0.0 0 0 0 0))
      (:SurfaceType3
        (goto _label)))))