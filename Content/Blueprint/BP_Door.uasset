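; BP_Door is a door that swings open when an XComCharacter overlaps its trigger.
; The OpenTrigger overlap plays the SWOpenDoor component on any overlap, then runs the DoorTimer timeline to yaw Door1 up to a scaled right angle.
; The construction script turns the OpeningDirection setting into a sign that picks the swing side.
; No closing logic exists, and other overlapping actors only print a failure message.
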(event OnComponentBeginOverlap(OpenTrigger)
  (params (OverlappedComponent :type Primitive%20Component%20Object%20Reference) (OtherActor :type Actor%20Object%20Reference) (OtherComp :type Primitive%20Component%20Object%20Reference) (OtherBodyIndex :type Integer) (bFromSweep :type Boolean) (SweepResult :type Hit%20Result%20Structure%20%28by%20ref%29))
  (Audio|Components|Audio|Play (Variables|Default|GetSW_OpenDoor) 0.0)
  ;[1 1 1] OPEN DOOR
  (Utilities|Casting|CastToXComCharacter OtherActor
    (:then
      (bind _doortimer (Timeline|DoorTimer Play)
        (:Update
          (Transformation|SetRelativeRotation (Variables|Default|GetDoor1) (Math|Rotator|MakeRotator 0.0 0.0 (* (* _doortimer 9e+01) (Variables|Default|GetDirection))) false false))))
    (:CastFailed
      (Development|PrintString "Failed" true true "(R=0.000000,G=0.660000,B=1.000000,A=1.000000)" 55.0))))

(event EventBeginPlay)

(event Collision|EventActorBeginOverlap
  (params (OtherActor :type Actor%20Object%20Reference)))

(event EventTick
  (params (DeltaSeconds :type Float%20%28single-precision%29)))

(fn ConstructionScript
  (switch Utilities|FlowControl|Switch|SwitchonENUM_OpeningDoor (Variables|Default|GetOpening_Direction)
    (:NewEnumerator0
      (Variables|Default|SetDirection -1.0))
    (:NewEnumerator1
      (Variables|Default|SetDirection 1.0))))