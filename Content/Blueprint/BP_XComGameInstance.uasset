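; BP_XComGameInstance is a game instance Blueprint with a LoadPlayerData event that spawns the player's hero characters.
; The event loops over the HerosCharacter array and spawns a new actor of each element's class at the world origin with default rotation and scale.
; It only takes the class from each stored hero, copying no other data, and prints debug messages with both actors' names.
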(event EventLoadPlayerData
  (Development|PrintString "Loadd" true true "(R=0.000000,G=0.660000,B=1.000000,A=1.000000)" 255.0)
  (for _array_element (Variables|Default|GetherosCharacter)
    (bind _returnvalue (Game|SpawnActorfromClass (Utilities|GetClass _array_element) (Math|Transform|MakeTransform "0, 0, 0") "Undefined" 0 0))
    (Development|PrintString "Load Player" true true "(R=0.000000,G=0.660000,B=1.000000,A=1.000000)" 55.0)
    (Development|PrintString (Utilities|GetDisplayName _returnvalue) true true "(R=0.000000,G=0.660000,B=1.000000,A=1.000000)" 55.0)
    (Development|PrintString (Utilities|GetDisplayName _array_element) true true "(R=0.000000,G=0.660000,B=1.000000,A=1.000000)" 55.0)))