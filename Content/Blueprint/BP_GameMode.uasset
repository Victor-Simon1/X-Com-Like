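; Game mode for a turn-based game with player-controlled heroes and enemies, tracking turn side, selected character and current target.
; On BeginPlay it attaches the UI and fills in player data, enemy count and turn number.
; Switching cycles possession through three BP_ParentHeros, updating selection and, via ChangePlayer, audio listener and UI, unless shooting.
; ChooseTarget cycles enemies by index, while SwitchEnnemie moves the hero's spring arm onto the current enemy.
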(event Custom|SwitchEnnemie
  (bind _asbp_parent_heros (Utilities|Casting|CastToBP_ParentHeros (Game|Player|GetPlayerPawn 0)))
  (Variables|/Game/Blueprint/BP_ParentHeros.BP_ParentHeros_C|SetOldLocation _asbp_parent_heros (Transformation|GetWorldLocation (Variables|/Script/Engine.Actor|GetRootComponent _asbp_parent_heros)))
  (bind _chosenactor (CallFunction|GetTarget1 (Variables|Default|GetCurrentEnnemieId)))
  (Transformation|SetWorldLocation (Variables|/Game/Blueprint/BP_ParentHeros.BP_ParentHeros_C|GetSpringArm _asbp_parent_heros) (Transformation|GetActorLocation _chosenactor) false false))

(event Custom|PossessPlayer
  ;[1 1 1] Switch character
  (bind _outactors (Actor|GetAllActorsOfClass "/Game/Blueprint/BP_ParentHeros.BP_ParentHeros_C"))
  (Pawn|Possess (Game|GetPlayerController 0) (Utilities|Array|Get(acopy) _outactors (Variables|Default|GetcurrentCharacterID)))
  (Class|BPCharacterInterface|Select(Message) (Utilities|Array|Get(acopy) _outactors (Variables|Default|GetcurrentCharacterID))))

(event Custom|Targeting
  (if (Variables|Default|GetPlayerIsShooting)
    (Variables|Default|SetHasChosen true)
    (Development|PrintString "Target Choose")
    (else
      (Development|PrintString "Player not shooting"))))

(event Custom|ChangePlayer
  (bind _returnvalue (Game|GetPlayerController 0))
  (if (not (Variables|Default|GetPlayerIsShooting))
    (if (< (Variables|Default|GetcurrentCharacterID) 2)
      (Variables|Default|SetcurrentCharacterID (+ (Variables|Default|GetcurrentCharacterID) 1))
      (else
        (Variables|Default|SetcurrentCharacterID 0)))
    (bind _asbp_game_mode (Utilities|Casting|CastToBP_GameMode (Game|GetGameMode)))
    (CallFunction|SetCharacterId _asbp_game_mode (Variables|Default|GetcurrentCharacterID))
    (bind _outactors (Actor|GetAllActorsOfClass "/Game/Blueprint/BP_ParentHeros.BP_ParentHeros_C"))
    (for (_array_element _array_index) _outactors
      (if (== _array_index (Variables|Default|GetcurrentCharacterID))
        (Pawn|Possess _returnvalue _array_element)
        (Class|BPCharacterInterface|Select(Message) _array_element)
        (Class|PlayerController|SetAudioListenerAttenuationOverride _returnvalue (Variables|/Script/Engine.Character|GetMesh _array_element) "0, 0, 0")
        (Default|SetData (Variables|Default|GetUI) _array_element)
        (else
          (Class|BPCharacterInterface|UnSelect(Message) _array_element))))))

(event EventBeginPlay
  (bind _returnvalue (Game|Player|GetPlayerPawn 0))
  (Variables|Default|SetPlayerTurn true)
  (Variables|Default|SetPlayerIsShooting false)
  (bind _ui (CallFunction|AttachUI))
  (bind _output_get (Variables|Default|SetUI _ui))
  (Default|SetData _output_get _returnvalue)
  (Default|SetHealthBar _output_get _returnvalue)
  (bind _outactors (Actor|GetAllActorsOfClass "/Game/Blueprint/BP_EnnemyCharacter.BP_EnnemyCharacter_C"))
  (bind _output_get_2 (Variables|Default|SetNBMaxEnnemie (Utilities|Array|Length _outactors)))
  (Default|SetTextEnnemieRestant (Variables|Default|GetUI) _output_get_2)
  (bind _output_get_3 (Variables|Default|SetCurrentTurn 1))
  (Default|SetTurnNumber (Variables|Default|GetUI) _output_get_3))

(event EventTick
  (params (DeltaSeconds :type Float%20%28single-precision%29)))

(fn ConstructionScript)

(fn ChangeTurn
  (bind _output_get (Variables|Default|SetPlayerTurn (not (Variables|Default|GetPlayerTurn))))
  (Default|SetView (Variables|Default|GetUI) _output_get)
  (return _output_get))

(fn PossessP
  ;[1 1 1] Switch character
  (if (< (Variables|Default|GetcurrentCharacterID) 2)
    (Variables|Default|SetcurrentCharacterID (+ (Variables|Default|GetcurrentCharacterID) 1))
    (else
      (Variables|Default|SetcurrentCharacterID 0)))
  (bind _outactors (Actor|GetAllActorsOfClass "/Game/Blueprint/BP_ParentHeros.BP_ParentHeros_C"))
  (for (_array_element _array_index) _outactors
    (if (== _array_index (Variables|Default|GetcurrentCharacterID))
      (Pawn|Possess (Game|GetPlayerController 0) _array_element)
      (Class|BPCharacterInterface|Select(Message) _array_element)
      (else
        (Class|BPCharacterInterface|UnSelect(Message) _array_element)))
    (return _array_element)))

(fn SetCharacterId
  (params (Id :type Integer))
  (Variables|Default|SetCurrentCharacterId Id))

(fn ChooseTarget
  (bind _currentidtarget (Variables|Default|GetCurrentIdTarget))
  (CallFunction|SetCurrentIdTarget)
  (bind _outactors (Actor|GetAllActorsOfClass "/Game/Blueprint/BP_EnnemyCharacter.BP_EnnemyCharacter_C"))
  (Development|PrintString (Utilities|String|ToString(Integer) _currentidtarget))
  (Default|SetData (Variables|Default|GetUI) (Utilities|Array|Get(acopy) _outactors _currentidtarget))
  (return (Utilities|Array|Get(acopy) _outactors _currentidtarget)))

(fn SetCurrentIdTarget
  (if (>= (Variables|Default|GetCurrentIdTarget) (- (Variables|Default|GetNBMaxEnnemie) 1))
    (Variables|Default|SetCurrentIdTarget 0)
    (else
      (Variables|Default|SetCurrentIdTarget (+ (Variables|Default|GetCurrentIdTarget) 1)))))

(fn GetTarget1
  (params (Id :type Integer))
  (bind _outactors (Actor|GetAllActorsOfClass "/Game/Blueprint/BP_EnnemyCharacter.BP_EnnemyCharacter_C"))
  (return (Utilities|Array|Get(acopy) _outactors Id)))