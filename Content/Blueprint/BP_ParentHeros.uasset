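; Parent hero character for a turn-based shooter, loading its stats, portrait and action points from a data table row on construction.
; Inputs work through BP_GameMode to switch hero or view another target, and to toggle move/shoot mode with camera and UI updates.
; Target is set only on entering shoot mode.
; Firing damages it if within range, turning the hero by timeline, and spends an action point even out of range.
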(event Custom|TimelineRotation
  (bind _alpha (Timeline|Timeline_0 Play)
    (:Update
      (CallFunction|RotatetoActor self (Variables|Default|Gettarget) _alpha))))

(event EventBeginPlay
  (|CallParentFunction))

(event Collision|EventActorBeginOverlap
  (params (OtherActor :type Actor%20Object%20Reference)))

(event EventTick
  (params (DeltaSeconds :type Float%20%28single-precision%29))
  (|CallParentFunction DeltaSeconds))

(event EventSelect
  ;[1 1 1] Select
)

(event EventUnSelect
  ;[1 1 1] UnSelect
)

(event Input|ActionEvents|InputActionShootMode
  (params (Key :type Key%20Structure :default "None"))
  ;[1 0.7983 0] When press p: pass to mode shoot <--> move
  (:Pressed
    (Development|PrintString "Shoot")
    (bind _asbp_game_mode (Utilities|Casting|CastToBP_GameMode (Game|GetGameMode)))
    (if (Variables|/Game/Blueprint/BP_GameMode.BP_GameMode_C|GetPlayerIsShooting _asbp_game_mode)
      (CallFunction|CamtoPlayer)
      (Variables|/Game/Blueprint/BP_GameMode.BP_GameMode_C|SetPlayerIsShooting _asbp_game_mode false)
      (Default|SetActionType (Variables|/Game/Blueprint/BP_GameMode.BP_GameMode_C|GetUI _asbp_game_mode))
      (Default|ShowTextDistanceShoot (Variables|/Game/Blueprint/BP_GameMode.BP_GameMode_C|GetUI _asbp_game_mode) true)
      (else
        (bind _chosenactor (Default|ChooseTarget _asbp_game_mode))
        (bind _asbp_ennemy_character (Utilities|Casting|CastToBP_EnnemyCharacter _chosenactor))
        (Variables|Default|Settarget _asbp_ennemy_character)
        (Default|CamtoTarget _asbp_game_mode _chosenactor self)
        (Variables|/Game/Blueprint/BP_GameMode.BP_GameMode_C|SetPlayerIsShooting _asbp_game_mode true)
        (Default|SetActionType (Variables|/Game/Blueprint/BP_GameMode.BP_GameMode_C|GetUI _asbp_game_mode) 1)
        (bind _dist (CallFunction|GetDisttoTarget _chosenactor))
        (bind _canshoot (CallFunction|VerifyDist _dist))
        (Default|ShowTextDistanceShoot (Variables|/Game/Blueprint/BP_GameMode.BP_GameMode_C|GetUI _asbp_game_mode) _canshoot)))))

(event Input|ActionEvents|InputActionSwitchPlayer/SwitchTarget
  (params (Key :type Key%20Structure :default "None"))
  ;[1 0.7798 0.06297] When press space : switch character
  (:Pressed
    (bind _asbp_game_mode (Utilities|Casting|CastToBP_GameMode (Game|GetGameMode)))
    (Variables|Default|SetcurrentZone 0)
    (Default|UpdateZone _asbp_game_mode)
    (if (Variables|/Game/Blueprint/BP_GameMode.BP_GameMode_C|GetPlayerTurn _asbp_game_mode)
      (if (Variables|/Game/Blueprint/BP_GameMode.BP_GameMode_C|GetPlayerIsShooting _asbp_game_mode)
        (bind _chosenactor (Default|ChooseTarget _asbp_game_mode))
        (Development|PrintString (Utilities|GetDisplayName _chosenactor))
        (Transformation|SetWorldLocation (Variables|Default|GetSpringArm) (Transformation|GetActorLocation _chosenactor) false false)
        (else
          (Default|ChangePlayer _asbp_game_mode)
          (Variables|/Script/Engine.MovementComponent|SetVelocity (Variables|Character|GetCharacterMovement) "0, 0, 0"))))))

(event Input|ActionEvents|InputActionFire
  (params (Key :type Key%20Structure :default "None"))
  ;[1 0.7416 0] When press enter : shoot
  (:Pressed
    (Development|PrintString "Je shoot dans l'ennemie" true true "(R=0.000000,G=0.660000,B=1.000000,A=1.000000)" 25.0)
    (bind _asbp_game_mode (Utilities|Casting|CastToBP_GameMode (Game|GetGameMode)))
    (if (Variables|/Game/Blueprint/BP_GameMode.BP_GameMode_C|GetPlayerIsShooting _asbp_game_mode)
      (CallFunction|ShootTemp (Variables|Default|Gettarget) 0.0)
      (bind _asbp_top_down_controller_2 (Utilities|Casting|CastToBP_TopDownController2 (Pawn|GetController)))
      (Default|ConsumePoint _asbp_top_down_controller_2 1)
      (else
        (Development|PrintString "Not shooting")))))

(fn ConstructionScript
  (bind _datatable (Variables|Default|GetdataTable))
  (bind (_datatable_2 _rowname) (Utilities|Struct|BreakDataTableRowHandle _datatable))
  (bind _returnvalue (Utilities|GetDataTableRow _datatable_2 _rowname)
    (:then
      (bind _output_get (Variables|Default|SethpMax (.hp (Utilities|Struct|BreakS_typePlayer _returnvalue))))
      (Variables|Default|Sethp _output_get)
      (Variables|Default|Setatk (.atk (Utilities|Struct|BreakS_typePlayer _returnvalue)))
      (Variables|Default|Setheal (.heal (Utilities|Struct|BreakS_typePlayer _returnvalue)))
      (Variables|Default|SetdistShoot (.distance_shoot (Utilities|Struct|BreakS_typePlayer _returnvalue)))
      (Variables|Default|Setpicture (.picture (Utilities|Struct|BreakS_typePlayer _returnvalue)))
      (Variables|Default|Settype (.type (Utilities|Struct|BreakS_typePlayer _returnvalue)))
      (Class|XComCharacter|SetMaxActionPoint (Math|Conversions|ToInteger(Byte) (.max_point_action (Utilities|Struct|BreakS_typePlayer _returnvalue)))))))

(fn ShootTemp
  (params (Target :type Actor%20Object%20Reference) (Alpha :type Float%20%28double-precision%29))
  (bind _returnvalue (Transformation|GetActorLocation))
  (bind _returnvalue_2 (Transformation|GetActorLocation Target))
  (bind _distshoot (Variables|Default|GetdistShoot))
  (bind _returnvalue_3 (- _returnvalue _returnvalue_2))
  (bind _returnvalue_4 (Math|Vector|VectorLength _returnvalue_3))
  (Development|PrintString (Utilities|String|ToString(Float) _returnvalue_4) true true "(R=0.000000,G=0.108595,B=1.000000,A=1.000000)" 255.0)
  (if (< _returnvalue_4 _distshoot)
    (CallFunction|TimelineRotation)
    (bind _asbp_ennemy_character (Utilities|Casting|CastToBP_EnnemyCharacter Target))
    (Class|XComCharacter|GetDamage _asbp_ennemy_character (Math|Float|Truncate (Variables|Default|Getatk)))
    (bind _asbp_game_mode (Utilities|Casting|CastToBP_GameMode (Game|GetGameMode)))
    (Default|SetData (Variables|/Game/Blueprint/BP_GameMode.BP_GameMode_C|GetUI _asbp_game_mode) _asbp_ennemy_character)
    (else
      (Development|PrintString "Trop loiun")
      (Development|PrintString (Utilities|String|ToString(Float) _distshoot)))))

(fn CamtoPlayer
  (Transformation|SetWorldLocation (Variables|Default|GetSpringArm) (Transformation|GetActorLocation self) false false))

(fn GetDisttoTarget
  (params (Target :type Actor%20Object%20Reference))
  (return (Math|Vector|Distance(Vector) (Transformation|GetActorLocation Target) (Transformation|GetActorLocation))))

(fn VerifyDist
  (params (Dist :type Float%20%28double-precision%29))
  (return (< Dist (Variables|Default|GetdistShoot))))