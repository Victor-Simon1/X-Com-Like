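; BP_ItemHp is a "Boost HP" pickup item that a hero consumes by walking into it.
; Its construction script creates an ItemHpBehavior object as the item's Behavior and sets the display name.
; On overlap with an XComHerosCharacter, it delegates the effect to that behavior's ConsumeItem, refreshes the game mode's UI with the character's data, then destroys itself.
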(event EventBeginPlay
  (|CallParentFunction))

(event Collision|EventActorBeginOverlap
  (params (OtherActor :type Actor%20Object%20Reference))
  (|CallParentFunction OtherActor)
  (bind _asxcom_heros_character (Utilities|Casting|CastToXComHerosCharacter OtherActor))
  (bind _asitem_hp_behavior (Utilities|Casting|CastToItemHpBehavior (Variables|Default|Getbehavior)))
  (Class|ItemBehavior|ConsumeItem _asitem_hp_behavior _asxcom_heros_character)
  (bind _asbp_game_mode (Utilities|Casting|CastToBP_GameMode (Game|GetGameMode)))
  (Default|SetData (Variables|/Game/Blueprint/BP_GameMode.BP_GameMode_C|GetUI _asbp_game_mode) _asxcom_heros_character)
  (Actor|DestroyActor))

(event EventTick
  (params (DeltaSeconds :type Float%20%28single-precision%29))
  (|CallParentFunction DeltaSeconds) ; This node is disabled and will not be called.\nDrag off pins to build functionality.
)

(fn ConstructionScript
  (|CallParentFunction)
  (bind _returnvalue (Game|ConstructObjectfromClass "/Script/XComLike.ItemHpBehavior"))
  (Variables|Default|Setbehavior _returnvalue)
  (Variables|Default|SetnameItem "Boost HP"))