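; Damage boost item Blueprint that adds to the player's "Boost DMG" utility count when an actor overlaps it.
; The construction script creates an ItemDmgBehavior object as its Behavior and sets the item name.
; On overlap, after the parent handler runs, it reaches the utilities panel widget through BP_GameMode, increments the count stored in that widget and refreshes its text.
; The overlap handler does not filter the overlapping actor.
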(event EventBeginPlay
  (|CallParentFunction))

(event Collision|EventActorBeginOverlap
  (params (OtherActor :type Actor%20Object%20Reference))
  (|CallParentFunction OtherActor)
  (bind _asbp_game_mode (Utilities|Casting|CastToBP_GameMode (Game|GetGameMode)))
  (bind _output_get (Variables|/Game/Blueprint/Interface/WB_Utilities.WB_Utilities_C|SetCountItem (Variables|/Game/Blueprint/Interface/WB_PanelUtilities.WB_PanelUtilities_C|GetWB_Utilities_DMG (Variables|/Game/Blueprint/Interface/WB_UI.WB_UI_C|GetWB_PanelUtilities (Variables|/Game/Blueprint/BP_GameMode.BP_GameMode_C|GetUI _asbp_game_mode))) (+ (Variables|/Game/Blueprint/Interface/WB_Utilities.WB_Utilities_C|GetCountItem (Variables|/Game/Blueprint/Interface/WB_PanelUtilities.WB_PanelUtilities_C|GetWB_Utilities_DMG (Variables|/Game/Blueprint/Interface/WB_UI.WB_UI_C|GetWB_PanelUtilities (Variables|/Game/Blueprint/BP_GameMode.BP_GameMode_C|GetUI _asbp_game_mode)))) 1)))
  (Rendering|Components|TextRender|SetText (Variables|/Game/Blueprint/Interface/WB_Utilities.WB_Utilities_C|GetCount (Variables|/Game/Blueprint/Interface/WB_PanelUtilities.WB_PanelUtilities_C|GetWB_Utilities_DMG (Variables|/Game/Blueprint/Interface/WB_UI.WB_UI_C|GetWB_PanelUtilities (Variables|/Game/Blueprint/BP_GameMode.BP_GameMode_C|GetUI _asbp_game_mode)))) (Utilities|Text|FormatText (Utilities|Text|ToText(String) (Utilities|String|ToString(Integer) _output_get)))))

(event EventTick
  (params (DeltaSeconds :type Float%20%28single-precision%29))
  (|CallParentFunction DeltaSeconds) ; This node is disabled and will not be called.\nDrag off pins to build functionality.
)

(fn ConstructionScript
  (|CallParentFunction)
  (bind _returnvalue (Game|ConstructObjectfromClass "/Script/XComLike.ItemDmgBehavior"))
  (Variables|Default|Setbehavior _returnvalue)
  (Variables|Default|SetnameItem "Boost DMG"))