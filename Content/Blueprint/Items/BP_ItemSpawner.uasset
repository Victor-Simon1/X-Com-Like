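; BP_ItemSpawner is a pickup actor that becomes a random item and is consumed when a hero overlaps it.
; On BeginPlay it picks a random DT_Item row, sets the mesh and constructs that row's Behavior object.
; On overlap with a BP_ParentHeros it delegates the effect to Behavior.ConsumeItem, refreshes the game mode's UI, logs the event and destroys itself.
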(event EventBeginPlay
  ;[1 1 1] Create random item
  (bind _outrownames (DataTable|GetDataTableRowNames "/Game/Blueprint/Items/DT_Item.DT_Item"))
  (bind _returnvalue (Utilities|GetDataTableRow "/Game/Blueprint/Items/DT_Item.DT_Item" (.OutItem (Utilities|Array|Random _outrownames)))
    (:then
      (Components|StaticMesh|SetStaticMesh (Variables|Default|GetStaticMesh) (.Mesh (Utilities|Struct|BreakS_Item _returnvalue)))
      (bind _returnvalue_2 (Game|ConstructObjectfromClass (.Behavior (Utilities|Struct|BreakS_Item _returnvalue))))
      (Variables|Default|Setbehavior _returnvalue_2))))

(event EventTick
  (params (DeltaSeconds :type Float%20%28single-precision%29)))

(event Collision|EventActorBeginOverlap
  (params (OtherActor :type Actor%20Object%20Reference))
  ;[1 1 1] Consume item
  (bind _asbp_parent_heros (Utilities|Casting|CastToBP_ParentHeros OtherActor))
  (Class|ItemBehavior|ConsumeItem (Variables|Default|GetBehavior) _asbp_parent_heros)
  (bind _asbp_game_mode (Utilities|Casting|CastToBP_GameMode (Game|GetGameMode)))
  (Default|SetData (Variables|/Game/Blueprint/BP_GameMode.BP_GameMode_C|GetUI _asbp_game_mode) _asbp_parent_heros)
  (CallFunction|AddLog "tEvent" "Item : added")
  (Actor|DestroyActor))

(fn ConstructionScript)